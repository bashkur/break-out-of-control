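; BP_Water_Ball is a water ball actor that plays a splash sound at its own location whenever its PlayNoise flag is set.
; Tick polls the flag, plays Splash_Cue at the root component's location and clears the flag.
; A DoOnce that resets after a short delay throttles repeat splashes.
; Nothing in this graph sets PlayNoise, and the construction script only calls its parent.
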(event EventBeginPlay
  (|CallParentFunction) ; This node is disabled and will not be called.\nDrag off pins to build functionality.
)

(event Collision|EventActorBeginOverlap
  (params (OtherActor :type Actor%20Object%20Reference))
  (|CallParentFunction OtherActor) ; This node is disabled and will not be called.\nDrag off pins to build functionality.
)

(event EventTick
  (params (DeltaSeconds :type Float%20%28single-precision%29))
  (|CallParentFunction DeltaSeconds)
  (if (Variables|Default|GetPlayNoise)
    (Utilities|FlowControl|DoOnce false :!label _label
      (:Completed
        (Audio|PlaySoundatLocation "/Game/Assets/Music_SFX/Splash_Cue.Splash_Cue" (Transformation|GetWorldLocation (Variables|Transformation|GetRootComponent)) "0, 0, 0" 1.0 1.0 0.0 0 0 0)
        (Variables|Default|SetPlayNoise false)
        (Utilities|FlowControl|Delay 0.5)
        (goto _label Reset)))))

(fn ConstructionScript
  (|CallParentFunction))