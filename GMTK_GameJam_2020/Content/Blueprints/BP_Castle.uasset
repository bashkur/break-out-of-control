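; BP_Castle is a castle actor with an HP value that gives audio feedback for impacts and destruction.
; Tick polls its state, playing the destroyed cue at the castle's location once when HP reaches zero or below.
; While HP remains, a raised PlayHitNoise flag triggers a wall-impact cue and is then cleared.
; The Blueprint itself never changes HP or raises that flag, and its other graphs are empty.
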(event EventBeginPlay)

(event Collision|EventActorBeginOverlap
  (params (OtherActor :type Actor%20Object%20Reference)))

(event EventTick
  (params (DeltaSeconds :type Float%20%28single-precision%29))
  (if (<= (Variables|Default|GetHP) 0.0)
    (Utilities|FlowControl|DoOnce false
      (:Completed
        (Audio|PlaySoundatLocation "/Game/Assets/Music_SFX/Castle_Destroyed_Cue.Castle_Destroyed_Cue" (Transformation|GetWorldLocation (Variables|Transformation|GetRootComponent)) "0, 0, 0" 1.0 1.0 0.0 0 0 0)))
    (elif (Variables|Default|GetPlayHitNoise)
      (Audio|PlaySoundatLocation "/Game/Assets/Music_SFX/Big_Wall_Impact_Cue.Big_Wall_Impact_Cue" (Transformation|GetWorldLocation (Variables|Transformation|GetRootComponent)) "0, 0, 0" 1.0 1.0 0.0 0 0 0)
      (Variables|Default|SetPlayHitNoise false))))

(fn ConstructionScript)

(fn NewFunction0)