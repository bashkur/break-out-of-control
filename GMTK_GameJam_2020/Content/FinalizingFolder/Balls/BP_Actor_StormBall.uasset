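; BP_Actor_StormBall is a storm ball visual actor with an outer ball and a core, whose active look is driven through materials.
; The construction script creates dynamic material instances for both parts and sets their bIsActive scalar to fully on.
; SetIsActive takes a value, clamps it between zero and one, and writes it to both materials.
; The event graph holds no logic.
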(event EventBeginPlay)

(event Collision|EventActorBeginOverlap
  (params (OtherActor :type Actor%20Object%20Reference)))

(event EventTick
  (params (DeltaSeconds :type Float%20%28single-precision%29)))

(fn ConstructionScript
  (bind _returnvalue (Rendering|Material|CreateDynamicMaterialInstance (Variables|Default|GetStormBall) 0 "/Game/Jeffs_Shader_Emporium/Storm_Ball_Src/fx_Storm_Ball_Mat.fx_Storm_Ball_Mat" "DynamicMat" :!class /Script/Engine.PrimitiveComponent))
  (bind _output_get (Variables|Default|SetDynamicStormBallMat _returnvalue))
  (Rendering|Material|SetScalarParameterValue _output_get "bIsActive" 1.0 :!class /Script/Engine.MaterialInstanceDynamic)
  (bind _returnvalue_2 (Rendering|Material|CreateDynamicMaterialInstance (Variables|Default|GetStormBall_Core) 0 "/Game/Jeffs_Shader_Emporium/Storm_Ball_Src/fx_Storm_Ball_Core_Mat.fx_Storm_Ball_Core_Mat" "DynamicMat" :!class /Script/Engine.PrimitiveComponent))
  (bind _output_get_2 (Variables|Default|SetDynamicStormBallCoreMat _returnvalue_2))
  (Rendering|Material|SetScalarParameterValue _output_get_2 "bIsActive" 1.0 :!class /Script/Engine.MaterialInstanceDynamic))

(fn SetIsActive
  (params (is_active :type Float%20%28single-precision%29))
  (bind _returnvalue (Math|Float|Clamp(Float) is_active))
  (Rendering|Material|SetScalarParameterValue (Variables|Default|GetDynamicStormBallMat) "bIsActive" _returnvalue :!class /Script/Engine.MaterialInstanceDynamic)
  (Rendering|Material|SetScalarParameterValue (Variables|Default|GetDynamicStormBallCoreMat) "bIsActive" _returnvalue :!class /Script/Engine.MaterialInstanceDynamic))