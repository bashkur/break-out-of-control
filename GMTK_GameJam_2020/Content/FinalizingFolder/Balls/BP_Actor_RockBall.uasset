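; BP_Actor_RockBall is a rock ball actor that spins and bobs in the world, with a material that shows an active state.
; Tick applies a fixed rotation and a sine-driven vertical offset to the RockBall component, neither scaled by delta time.
; The construction script creates a dynamic material from Fx_Rock_Ball_Mat with bIsActive on.
; SetIsActive writes a clamped zero-to-one value to that parameter.
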(event EventBeginPlay)

(event EventTick
  (params (DeltaSeconds :type Float%20%28single-precision%29))
  (Transformation|AddWorldRotation (Variables|Default|GetRockBall) "0,1.000000, 0" false false)
  (bind _output_get (Variables|Default|SetElapsedTime (+ DeltaSeconds (Variables|Default|GetElapsedTime))))
  (Transformation|AddWorldOffset (Variables|Default|GetRockBall) (Math|Vector|MakeVector 0.0 0.0 (* (Math|Trig|Sin(Radians) _output_get) 0.25)) false false))

(fn ConstructionScript
  (bind _returnvalue (Rendering|Material|CreateDynamicMaterialInstance (Variables|Default|GetRockBall) 0 "/Game/Jeffs_Shader_Emporium/Rock_Ball_Src/fx_Rock_Ball_Mat.fx_Rock_Ball_Mat" "DyanmicMat" :!class /Script/Engine.PrimitiveComponent))
  (bind _output_get (Variables|Default|SetDynamicRockBallMat _returnvalue))
  (Rendering|Material|SetScalarParameterValue _output_get "bIsActive" 1.0 :!class /Script/Engine.MaterialInstanceDynamic))

(fn SetIsActive
  (params (is_active :type Float%20%28single-precision%29))
  (Rendering|Material|SetScalarParameterValue (Variables|Default|GetDynamicRockBallMat) "bIsActive" (Math|Float|Clamp(Float) is_active) :!class /Script/Engine.MaterialInstanceDynamic))